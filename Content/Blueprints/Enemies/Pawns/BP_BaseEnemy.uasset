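; BP_BaseEnemy is a base enemy that carries a weapon and dies when its health runs out.
; On BeginPlay it spawns a BP_Weapon and snaps it to the hand_rSocket on its mesh.
; SetDamage subtracts the received damage from Health, prints the result and updates the death flag.
; Once health reaches zero or below, it destroys both itself and the weapon.
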(event `self.ReceiveBeginPlay`
  (bind _returnvalue (`|SpawnActorFromClass` "/Game/Blueprints/Enemies/BP_Weapon.BP_Weapon_C" (`SceneComponent.K2_GetComponentToWorld` (`self.Mesh`)) "AlwaysSpawn" "OverrideRootScale" null null))
  (bind _output_get (set `self.weapon` _returnvalue))
  (`self.K2_AttachToComponent` _output_get (`self.Mesh`) "hand_rSocket" "SnapToTarget" "SnapToTarget" "SnapToTarget" true))

(event `/Game/Blueprints/Interface.setDamage`
  (params (damageRecieved :type "Float (single-precision)"))
  (`self.calculateHealth` damageRecieved)
  (if (`self.isDeath?`)
    (`self.K2_DestroyActor` self)
    (`self.K2_DestroyActor` (`self.weapon`))))

(fn `calculateDeath`
  (if (<= (`self.health`) 0.0)
    (set `self.isDeath?` true)
    (else
      (set `self.isDeath?` false))))

(fn `calculateHealth`
  (params (damage :type "Float (double-precision)"))
  (bind _output_get (set `self.health` (- (`self.health`) damage)))
  (`KismetSystemLibrary.PrintString` (`KismetStringLibrary.Conv_DoubleToString` _output_get))
  (`self.calculateDeath`))

(fn `UserConstructionScript`)