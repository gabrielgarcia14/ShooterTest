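; AI controller for enemies that runs the BT_Enemies behavior tree when it possesses a BP_BaseEnemy.
; When perception updates on the player, it writes the sensed state to the "canSeeHim?" blackboard key and prints it.
; The same update pulls or releases the controlled enemy's weapon trigger directly, outside the tree.
; A DirectMovement graph holds unconnected timer and AIMoveTo nodes for chasing the player, which never run.
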(event `findingPlayer`)

(event `self.ReceiveBeginPlay`)

(event `self.ReceivePossess`
  (params (PossessedPawn :type "Pawn Object Reference"))
  (cast `/Game/Blueprints/Enemies/Pawns/BP_BaseEnemy` PossessedPawn)
  (`self.RunBehaviorTree` "/Game/Blueprints/Enemies/AI/BT_Enemies.BT_Enemies"))

(event `self.AIPerception.OnTargetPerceptionUpdated`
  (params (Actor :type "Actor Object Reference") (Stimulus :type "AIStimulus Structure"))
  (bind (_age _expirationage _strength _stimuluslocation _receiverlocation _tag _bsuccessfullysensed) (break `AIStimulus` Stimulus))
  (bind _returnvalue (`self.K2_GetPawn`))
  (cast `/Game/Blueprints/BP_Player` Actor)
  (`BlackboardComponent.SetValueAsBool` (`AIBlueprintHelperLibrary.GetBlackboard` null) "canSeeHim?" _bsuccessfullysensed)
  (`KismetSystemLibrary.PrintString` (`KismetStringLibrary.Conv_BoolToString` _bsuccessfullysensed))
  (if _bsuccessfullysensed
    (bind _asbp_base_enemy (cast `/Game/Blueprints/Enemies/Pawns/BP_BaseEnemy` _returnvalue))
    (`/Game/Blueprints/Enemies/BP_Weapon.pullTrigger` (`/Game/Blueprints/Enemies/Pawns/BP_BaseEnemy.weapon` _asbp_base_enemy))
    (else
      (bind _asbp_base_enemy_2 (cast `/Game/Blueprints/Enemies/Pawns/BP_BaseEnemy` _returnvalue))
      (`/Game/Blueprints/Enemies/BP_Weapon.releaseTrigger` (`/Game/Blueprints/Enemies/Pawns/BP_BaseEnemy.weapon` _asbp_base_enemy_2)))))

(fn `UserConstructionScript`)